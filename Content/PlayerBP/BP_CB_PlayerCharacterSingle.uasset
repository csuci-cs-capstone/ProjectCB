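; Single-player character Blueprint that adds pause menu handling on the P key.
; PauseGame creates a new PauseMenu widget, adds it to the viewport and switches to UI-only input, without pausing game time.
; UnpauseGame removes all widgets and restores game-only input; both functions keep the mouse cursor hidden.
; The capsule debug draw and the check for reusing an existing menu are disconnected.
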(event EventBeginPlay)

(event Collision|EventActorBeginOverlap
  (params (OtherActor :type Actor%20Object%20Reference)))

(event EventTick
  (params (DeltaSeconds :type Float%20%28single-precision%29))
  ;[1 1 1] Capsule Debug
)

(event Input|KeyboardEvents|P
  (params (Key :type Key%20Structure :default "None"))
  ;[1 1 1] Pause Game
  (:Pressed
    (CallFunction|PauseGame)))

(fn ConstructionScript)

(fn PauseGame
  (bind _returnvalue (UserInterface|CreateWidget "/Game/WorldBP/PauseMenu.PauseMenu_C" (Game|GetPlayerController 0)))
  (Variables|Default|SetPauseMenu _returnvalue)
  (UserInterface|Viewport|AddtoViewport (Variables|Default|GetPauseMenu) 0)
  (Input|SetInputModeUIOnly (Game|GetPlayerController 0) (Variables|Default|GetPauseMenu) "DoNotLock")
  (Variables|/Script/Engine.PlayerController|SetbShowMouseCursor (Game|GetPlayerController 0) false))

(fn UnpauseGame
  (bind _returnvalue (Game|GetPlayerController 0))
  (Viewport|RemoveAllWidgets)
  (Input|SetInputModeGameOnly _returnvalue)
  (Variables|/Script/Engine.PlayerController|SetbShowMouseCursor _returnvalue false))